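; BP_Bullet is a projectile that moves itself every frame in a straight line based on its rotation.
; Tick rotates the actor's forward vector -90 degrees around world Y, scales it by Speed and adds it to the location.
; The step is not scaled by DeltaSeconds and does not sweep, so travel depends on frame rate and ignores blocking.
; Hit handling is absent, and leftover speed and rotation nodes never run.
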(event EventBeginPlay)

(event Collision|EventActorBeginOverlap
  (params (OtherActor :type Actor%20Object%20Reference)))

(event EventTick
  (params (DeltaSeconds :type Float%20%28single-precision%29))
  (Variables|Default|SetDeltaSeconds DeltaSeconds)
  (Transformation|SetActorLocation (+ (Transformation|GetActorLocation) (* (Math|Vector|RotateVectorAroundAxis (Math|Rotator|GetRotationXVector (Transformation|GetActorRotation)) -9e+01 "0,1.000000, 0") (Variables|Default|GetSpeed))) false false))

(fn ConstructionScript)