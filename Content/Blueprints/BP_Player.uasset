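; BP_Player is a flying player character with thrust, inertia, gravity and projectile fire, introduced by a rising, spinning spawn timeline.
; The up axis eases thrust through FInterpTo, while the right axis pitches the actor.
; Tick sweeps it along its rotated forward vector plus a clamped momentum vector, which accumulates thrust and gravity and prints for debugging.
; Primary fire spawns BP_Bullet at ProjectileSpawn on press and again via a short timer.
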(event Custom|PrimFire
  (CallFunction|PrimaryFire (Transformation|GetWorldTransform (Variables|Default|GetProjectileSpawn)) (Math|Rotator|GetRotationXVector (Transformation|GetActorRotation))))

(event EventBeginPlay
  ;[1 1 1] Player spawn animation
  (bind _asbp_game_mode (Utilities|Casting|CastToBP_GameMode (Game|GetGameMode)))
  (Variables|Default|SetBP_GameMode _asbp_game_mode)
  (Variables|Default|SetYaw (.Yaw (Math|Rotator|BreakRotator (Transformation|GetActorRotation))))
  (Variables|Default|SetSpawnLocation (Transformation|GetActorLocation))
  (bind _speed (Timeline|SpawnAnimation Play)
    (:Update
      (Transformation|SetActorLocation (Math|Vector|Lerp(Vector) (Variables|Default|GetSpawnLocation) (+ (Variables|Default|GetSpawnLocation) "0, 0,60.000000") _speed) false false)
      (Transformation|SetActorRotation (Math|Rotator|Lerp(Rotator) "0, 0, 0" (Math|Rotator|MakeRotator 0.0 0.0 (+ (Variables|Default|GetYaw) (Variables|Default|GetSpawnSpinCount))) _speed)))
    (:Finished
      (Variables|Default|SetMoveEnabled true))))

(event EventTick
  (params (DeltaSeconds :type Float%20%28single-precision%29))
  (bind _returnvalue (Transformation|GetActorRotation))
  (bind _verticalspeed (Variables|Default|GetVerticalSpeed))
  (bind _movementmass (Variables|Default|GetMovementMass))
  (bind _returnvalue_2 (Math|Rotator|GetRotationXVector _returnvalue))
  (bind _returnvalue_3 (+ _movementmass _verticalspeed))
  (bind _returnvalue_4 (* _returnvalue_2 _returnvalue_3))
  (bind _returnvalue_5 (Math|Vector|RotateVectorAroundAxis _returnvalue_4 -9e+01 "0,1.000000, 0"))
  ;[1 1 1] transforming player based on speed
  (Variables|Default|SetDeltaSeconds DeltaSeconds)
  (Transformation|SetActorLocation (+ (Transformation|GetActorLocation) _returnvalue_5 (stale _output_get)) true false)
  (bind _output_get (Variables|Default|SetMovementMassVector (Math|Vector|ClampVectorSize (+ (* _returnvalue_5 0.1) (Variables|Default|GetMovementMassVector) (* (Math|Vector|VectorDown) (Variables|Default|GetGravity))) 0.0 3.0)))
  (Development|PrintString (Utilities|String|ToString(Vector) _output_get)))

(event Input|ActionEvents|InputActionPrimaryFire
  (params (Key :type Key%20Structure :default "None"))
  (:Pressed
    (Utilities|Time|SetTimerbyFunctionName 0 "PrimFire" 0.2)
    (CallFunction|PrimaryFire (Transformation|GetWorldTransform (Variables|Default|GetProjectileSpawn)) (Math|Rotator|GetRotationXVector (Transformation|GetActorRotation)))))

(event Input|AxisEvents|InputAxisMoveUp
  (params (AxisValue :type Float%20%28single-precision%29))
  ;[1 1 1] Smooth speed acceleration for input
  (bind _returndirectionspeed (CallFunction|Movement AxisValue (Variables|Default|GetVerticalSpeed)))
  (bind _output_get (Variables|Default|SetVerticalSpeed _returndirectionspeed)))

(event Input|AxisEvents|InputAxisMoveRight
  (params (AxisValue :type Float%20%28single-precision%29))
  ;[1 1 1] Smooth speed acceleration for input
  (Transformation|AddActorLocalRotation (Math|Rotator|MakeRotator 0.0 (* AxisValue 2.7) 0.0) false false))

(fn ConstructionScript)

(fn Movement
  (params (Direction :type Float%20%28single-precision%29) (Speed :type Float%20%28single-precision%29))
  (return (Math|Interpolation|FInterpTo Speed (* (Variables|Default|GetMovementSpeed) Direction) (Variables|Default|GetDeltaSeconds) 5.0)))

(fn PrimaryFire
  (params (SpawnTransform :type Transform) (Rotation :type Vector))
  (Game|SpawnActorfromClass "/Game/Blueprints/BP_Bullet.BP_Bullet_C" SpawnTransform "AlwaysSpawn" 0 self))